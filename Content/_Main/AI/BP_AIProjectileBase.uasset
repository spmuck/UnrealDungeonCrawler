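; Base AI projectile that damages the first living player its collision sphere overlaps.
; Overlaps resolve on the authority: tagged players are checked for death state through a message call, enemies are ignored, and other actors cause impact without damage.
; Impacts play particle and sound through a Multi_PlayHitFx event, then destroy the projectile after a short delay.
; A stored HitPlayer blocks further hits once a player is struck.
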(event `self.Sphere.OnComponentBeginOverlap`
  (params (OverlappedComponent :type "PrimitiveComponent Object Reference") (OtherActor :type "Actor Object Reference") (OtherComp :type "PrimitiveComponent Object Reference") (OtherBodyIndex :type Integer) (bFromSweep :type Boolean) (SweepResult :type "HitResult Structure (by ref)"))
  (bind (_bblockinghit _binitialoverlap _time _distance _location) (`GameplayStatics.BreakHitResult` SweepResult))
  (`self.HitPlayer`
    (:`then`)
    (:`else`
      (`/Engine/EditorBlueprintResources/ActorMacros.Switch Has Authority`
        (:`Authority`
          (if (`self.ActorHasTag` OtherActor "Player")
            (bind _state (message `/Game/_Main/Interfaces/INT_PlayerCharacter.PlayerDeathState` OtherActor))
            (if (not _state)
              (set `self.HitPlayer` OtherActor)
              (bind _output_get (set `self.HitLocation` _location))
              (`self.Multi_PlayHitFx` (`self.HitParticle`) _output_get (`self.HitScale`) (`self.HitSound`))
              (`GameplayStatics.ApplyDamage` (`self.HitPlayer`) (`self.Damage`) null (`self.GetOwner`) "/Script/Engine.DamageType")
              (`KismetSystemLibrary.Delay` 0.1)
              (`self.K2_DestroyActor`))
            (elif (not (`self.ActorHasTag` OtherActor "Enemy"))
              (`self.Multi_PlayHitFx` (`self.HitParticle`) _location (`self.HitScale`) (`self.HitSound`))
              (`KismetSystemLibrary.Delay` 0.1)
              (`self.K2_DestroyActor`))))))))

(event `Multi_PlayHitFx`
  (params (EmitterTemplate :type "ParticleSystem Object Reference") (Location :type "Vector Structure") (Scale :type "Vector Structure") (Sound :type "SoundBase Object Reference"))
  (`GameplayStatics.SpawnEmitterAtLocation` EmitterTemplate Location (struct) Scale)
  (`GameplayStatics.PlaySoundAtLocation` Sound Location (struct) 1.0 1.0 0.0 null null null))

(fn `UserConstructionScript`)