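; Base enemy character that chases a player target, attacks it, and heads back to its spawn location when the target is cleared.
; SetNewTarget starts an AIMoveTo chase and attack loop that plays random montage sections in range, pausing between attacks.
; Tick, switched on for combat, yaws the enemy toward its target.
; Death clears the target, stuns feed back into the chase, and AIRangeAttack spawns projectiles on authority.
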(event `self.ReceiveBeginPlay`
  (`self.f_MovementState` "NewEnumerator0")
  (set `self.SpawnedLocation` (`self.K2_GetActorLocation`)))

(event `/Game/_Main/Interfaces/INT_EnemyBase.Set New Target`
  (params (PlayerTarget :type "Pawn Object Reference"))
  ;[1 1 1] sets player target if it hasn't been set
  (`self.PlayerTarget`
    (:`then`)
    (:`else`
      (bind _state (message `/Game/_Main/Interfaces/INT_PlayerCharacter.PlayerDeathState` PlayerTarget))
      (if (not _state)
        (set `self.PlayerTarget` PlayerTarget)
        (set `self.InCombat` true)
        (`self.SetActorTickEnabled` true)
        (`self.f_MovementState` "NewEnumerator1")
        (`self.ChasePlayer`)))))

(event `ChasePlayer`
  (if (and (`self.InCombat`) (not (`self.isStuned`)))
    (`|AIMoveTo` self (0.0 0.0 0.0) (`self.PlayerTarget`) (`self.AcceptanceRadius`)
      (:`OnSuccess`
        (`self.AttackPlayer`)))))

(event `self.ReceiveTick`
  (params (DeltaSeconds :type "Float (single-precision)"))
  (bind (_returnvalue_roll _returnvalue_pitch _returnvalue_yaw) (`KismetMathLibrary.BreakRotator` (`KismetMathLibrary.FindLookAtRotation` (`self.K2_GetActorLocation`) (`self.K2_GetActorLocation` (`self.PlayerTarget`)))))
  ;[1 1 1] Rotate player when in combat
  (`self.PlayerTarget`
    (:`then`
      (if (and (`self.InCombat`) (not (`self.isStuned`)))
        (`self.K2_SetActorRotation` (`KismetMathLibrary.MakeRotator` 0.0 0.0 _returnvalue_yaw))))
    (:`else`
      (`self.SetActorTickEnabled` false)
      (`self.AttackPlayer`))))

(event `AttackPlayer`
  (if (and (not (`self.isDead`)) (not (`self.isStuned`)))
    (bind _state (message `/Game/_Main/Interfaces/INT_PlayerCharacter.PlayerDeathState` (`self.PlayerTarget`)))
    (if (not _state)
      (bind _output_get (set `self.DistanceToPlayer` (`self.GetDistanceTo` (`self.PlayerTarget`))))
      (if (<= _output_get (`self.AttackRange`))
        (`self.f_PlayAttackMontage`)
        (`KismetSystemLibrary.Delay` (`self.TimeBetweenAttacks`))
        (`self.ChasePlayer`)
        (else
          (`self.ChasePlayer`)))
      (else
        (`self.ClearTarget`)))))

(event `/Game/_Main/Interfaces/INT_EnemyBase.AIRangeAttack`
  (bind _projectilearrow (`self.ProjectileArrow`))
  (`/Engine/EditorBlueprintResources/ActorMacros.Switch Has Authority`
    (:`Authority`
      (`|SpawnActorFromClass` (`self.Projectile`) (`KismetMathLibrary.MakeTransform` (`SceneComponent.K2_GetComponentLocation` _projectilearrow) (`SceneComponent.K2_GetComponentRotation` _projectilearrow)) "Undefined" "OverrideRootScale" self self))))

(event `ClearTarget`
  ;[1 1 1] Clears Player Target
  (set `self.InCombat` false)
  (`self.SetActorTickEnabled` false)
  (set `self.PlayerTarget` null)
  (if (not (`self.isDead`))
    (`|AIMoveTo` self (`self.SpawnedLocation`) null 20.0)))

(event `self.KillCharacter`
  (`parent.KillCharacter`)
  (`self.ClearTarget`))

(event `/Game/_Main/Interfaces/INT_BaseCharacter.StunCharacter`
  (params (StunDuration :type "Float (single-precision)"))
  (`parent.StunCharacter` StunDuration)
  (`self.ChasePlayer`))

(fn `f_MovementState`
  (params (State :type "/Game/_Main/AI/E_AIMovementState Enum" :default "NewEnumerator0"))
  (switch `/Game/_Main/AI/E_AIMovementState` State
    (:`NewEnumerator0`
      (set `self.TempWalkSpeed` 0.0))
    (:`NewEnumerator1`
      (set `self.TempWalkSpeed` (`self.WalkSpeed`)))
    (:`NewEnumerator2`
      (set `self.TempWalkSpeed` (`self.RunSpeed`))))
  (set `CharacterMovementComponent.MaxWalkSpeed` (`self.TempWalkSpeed`) (`self.CharacterMovement`)))

(fn `f_PlayAttackMontage`
  (bind _attacksection (`self.f_GetRandomAttackSection`))
  (`self.Multi_PlayMontageAndSound` (`self.Mesh`) (`self.AttackMontage`) _attacksection (`self.AttackSound`)))

(fn `UserConstructionScript`
  (`parent.UserConstructionScript`))