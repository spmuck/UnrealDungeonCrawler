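; PC_DungeonController is the player controller for the dungeon game, handling player lives, respawning, movement input and the player's UI.
; On BeginPlay it caches the controlled pawn and its stats, then creates the HUD widget for the local controller.
; Respawning spends a life, spawns and possesses a new pawn, and copies its stats to SavedStats, refreshing the UI, or prints game over.
; Move axis input drives the pawn along control-rotation vectors while movement is enabled.
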(event `ReplicateNewPlayerStats`
  (params (NewPlayerPawn :type "Object Object Reference"))
  (bind _stats (message `/Game/_Main/Interfaces/INT_PlayerCharacter.GetPlayerStats` NewPlayerPawn))
  (`self.SetSavedStats` _stats))

(event `self.SetSavedStats`
  (params (SavedStats :type "/Game/_Main/S_Stats Structure"))
  (set `self.SavedStats` SavedStats)
  (bind _playerui (`self.PlayerUI`)
    (:`then`
      (`/Game/_Main/UI/PlayerUI.UpdateDisplayedStats` _playerui (`self.SavedStats`)))
    (:`else`)))

(event `self.RespawnPlayer`
  (params (SpawnLocation :type "Vector Structure") (PlayerClass :type "/Game/_Main/BP_PlayerBase Class Reference"))
  (`self.DecreaseLives`)
  (if (>= (`self.Lives`) 0)
    (bind _returnvalue (`|SpawnActorFromClass` PlayerClass (`KismetMathLibrary.MakeTransform` (+ SpawnLocation (0.0 0.0 150.0))) "Undefined" "OverrideRootScale" null null))
    (`self.Possess` _returnvalue)
    (bind _output_get (set `self.PlayerPawn` _returnvalue))
    (`self.ReplicateNewPlayerStats` _output_get)
    (else
      (`KismetSystemLibrary.PrintString` "GAME OVER YOU DUMB BITCH"))))

(event `self.DecreaseLives`
  (`/Engine/EditorBlueprintResources/StandardMacros.DecrementInt` (`self.Lives`)))

(event `self.IncreaseLives`
  (`/Engine/EditorBlueprintResources/StandardMacros.IncrementInt` (`self.Lives`)))

(event `self.SetMovementEnabled`
  (params (MovementEnabled :type Boolean))
  (set `self.MovementEnabled` MovementEnabled))

(event `self.ReceiveBeginPlay`
  (`KismetSystemLibrary.Delay` 0.2)
  (set `self.PlayerPawn` (`self.K2_GetPawn`))
  (bind _stats (message `/Game/_Main/Interfaces/INT_PlayerCharacter.GetPlayerStats` (`self.PlayerPawn`)))
  (set `self.SavedStats` _stats)
  (if (`self.IsLocalController`)
    (bind _returnvalue (`|CreateWidget` "/Game/_Main/UI/PlayerUI.PlayerUI_C"))
    (bind _output_get (set `self.PlayerUI` _returnvalue))
    (`UserWidget.AddToViewport` _output_get 0)))

(event `InputAxis|MoveForward`
  (params (AxisValue :type "Float (single-precision)"))
  (bind _playerpawn (`self.PlayerPawn`))
  (`self.PlayerPawn`
    (:`then`
      (if (`self.MovementEnabled`)
        (`Pawn.AddMovementInput` _playerpawn (`KismetMathLibrary.GetForwardVector` (`Pawn.GetControlRotation` _playerpawn)) AxisValue false)))
    (:`else`)))

(event `InputAxis|MoveRight`
  (params (AxisValue :type "Float (single-precision)"))
  (bind _playerpawn (`self.PlayerPawn`))
  (`self.PlayerPawn`
    (:`then`
      (if (`self.MovementEnabled`)
        (`Pawn.AddMovementInput` _playerpawn (`KismetMathLibrary.GetRightVector` (`Pawn.GetControlRotation` _playerpawn)) AxisValue false)))
    (:`else`)))

(fn `GetSavedStats`
  (returns (Stats :type "/Game/_Main/S_Stats Structure"))
  (return (`self.SavedStats`)))

(fn `UserConstructionScript`)