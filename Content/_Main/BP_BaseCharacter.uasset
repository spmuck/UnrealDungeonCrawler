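; Base character Blueprint providing shared combat logic: montage attacks, blocking, damage, death, stun and mana spending, with Multi_ events and an OnRep for networking.
; AnyDamage ignores hits while blocking a frontal causer (2D dot-product test), otherwise reduces health and triggers death, delayed respawn and destruction.
; Stat changes go to the controller through interface messages, which also toggle movement around montage notifies.
; Block FX is a placeholder meant for overriding.
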(event `self.ReceivePossessed`
  (params (NewController :type "Controller Object Reference"))
  (set `self.ControllerRef` NewController))

(event `Multi_PlayMontageAndSound`
  (params (InSkeletalMeshComponent :type "SkeletalMeshComponent Object Reference") (MontageToPlay :type "AnimMontage Object Reference") (StartingSection :type Name) (AttackSound :type "SoundBase Object Reference"))
  (set `self.CurrentlyAttacking` true)
  (message `/Game/_Main/Interfaces/INT_PlayerController.SetMovementEnabled` (`self.ControllerRef`) false)
  (`|PlayMontage` InSkeletalMeshComponent MontageToPlay 1.0 0.0 StartingSection
    (:`OnNotifyBegin`
      (`GameplayStatics.PlaySoundAtLocation` AttackSound (`self.K2_GetActorLocation`) (struct) 1.0 1.0 0.0 null null null))
    (:`OnNotifyEnd`
      (set `self.CurrentlyAttacking` false)
      (message `/Game/_Main/Interfaces/INT_PlayerController.SetMovementEnabled` (`self.ControllerRef`) true))))

(event `Multi_PlayHitSound`
  (params (Sound :type "SoundBase Object Reference") (Location :type "Vector Structure"))
  (`GameplayStatics.PlaySoundAtLocation` Sound Location (struct) 1.0 1.0 0.0 null null null))

(event `Multi_BlockFX`
  (`KismetSystemLibrary.PrintString` "Blocked. Overwrite Multi_BlockFX to change behavior."))

(event `self.ReceiveAnyDamage`
  (params (Damage :type "Float (single-precision)") (DamageType :type "DamageType Object Reference") (InstigatedBy :type "Controller Object Reference") (DamageCauser :type "Actor Object Reference"))
  ;[1 1 1] Handle Damage
  (if (`self.IsBlocking`)
    (bind _isinfrontof (`self.f_IsTargetInfrontOfPlayer` DamageCauser))
    (if _isinfrontof
      (`self.Multi_BlockFX`)
      (else
        (`KismetSystemLibrary.PrintString` (`KismetStringLibrary.Conv_DoubleToString` Damage) :!label _label)
        (bind _structout (setmembers `/Game/_Main/S_Stats` :`StructRef` (`self.Stats`) :`CurrentHealth` (- (`.CurrentHealth_8_2A9736CB4B7A2C8C60B493B03620AC42` (break `/Game/_Main/S_Stats` (`self.Stats`))) Damage)))
        (`self.UpdateUIStats` _structout)
        (if (<= (`.CurrentHealth_8_2A9736CB4B7A2C8C60B493B03620AC42` (break `/Game/_Main/S_Stats` _structout)) 0.0)
          (`self.KillCharacter`))))
    (else
      (goto _label))))

(event `KillCharacter`
  ;[1 1 1] Handle Death
  (set `self.isDead` true)
  (`CharacterMovementComponent.DisableMovement` (`self.CharacterMovement`))
  (`self.Multi_Death`)
  (`CharacterMovementComponent.SetAvoidanceEnabled` (`self.CharacterMovement`) false)
  (`KismetSystemLibrary.Delay` 3.0)
  (message `/Game/_Main/Interfaces/INT_PlayerCharacter.RespawnCharacter` self)
  (`KismetSystemLibrary.Delay` 5.0)
  (`self.K2_DestroyActor`))

(event `Multi_Death`
  ;[1 1 1] Handle Death
  (`PrimitiveComponent.SetCollisionProfileName` (`self.CapsuleComponent`) "Ragdoll" true)
  (`self.StopAnimMontage` null)
  (message `/Game/_Main/Interfaces/INT_AnimBP.KillCharacter` (`SkeletalMeshComponent.GetAnimInstance` (`self.Mesh`))))

(event `UpdateUIStats`
  (params (StatsToSave :type "/Game/_Main/S_Stats Structure"))
  (message `/Game/_Main/Interfaces/INT_PlayerController.SetSavedStats` (`self.GetController`) StatsToSave))

(event `/Game/_Main/Interfaces/INT_BaseCharacter.StunCharacter`
  (params (StunDuration :type "Float (single-precision)"))
  (set `self.isStuned` true)
  (`KismetSystemLibrary.Delay` StunDuration)
  (set `self.isStuned` false))

(fn `f_GetRandomAttackSection`
  (returns (AttackSection :type Name))
  (bind _attacksections (`self.AttackSections`))
  (return (`|GetArrayItem` _attacksections (`KismetMathLibrary.RandomInteger` (`KismetArrayLibrary.Array_Length` _attacksections)))))

(fn `f_IsTargetInfrontOfPlayer`
  (params (TargetActor :type "Actor Object Reference"))
  (returns (IsInFrontOf :type Boolean))
  (bind (_returnvalue_x _returnvalue_y) (`KismetMathLibrary.BreakVector` (`self.GetActorForwardVector`)))
  (bind (_returnvalue_x_2 _returnvalue_y_2) (`KismetMathLibrary.BreakVector` (`KismetMathLibrary.GetDirectionUnitVector` (`self.K2_GetActorLocation` TargetActor) (`self.K2_GetActorLocation`))))
  (return (<= (`KismetMathLibrary.Dot_VectorVector` (`KismetMathLibrary.Normal` (`KismetMathLibrary.MakeVector` _returnvalue_x _returnvalue_y)) (`KismetMathLibrary.Normal` (`KismetMathLibrary.MakeVector` _returnvalue_x_2 _returnvalue_y_2))) -0.4)))

(fn `f_TryCastManaSpell`
  (params (ManaCost :type "Float (double-precision)"))
  (returns (CanCast :type Boolean))
  (locals (HasEnoughMana :type Boolean :default false) (NewMana :type "Float (double-precision)" :default 0.0))
  (bind _output_get (set `local.NewMana` (- (`.CurrentMana_10_2FF5416A4CB71095FDC09B9871DC1D76` (break `/Game/_Main/S_Stats` (`self.Stats`))) ManaCost)))
  (bind _output_get_2 (set `local.HasEnoughMana` (>= _output_get 0.0)))
  (if _output_get_2
    (bind _structout (setmembers `/Game/_Main/S_Stats` :`StructRef` (`self.Stats`) :`CurrentMana` (`local.NewMana`)))
    (`self.UpdateUIStats` _structout))
  (return (`local.HasEnoughMana`)))

(fn `OnRep_IsBlocking`
  (message `/Game/_Main/Interfaces/INT_AnimBP.SetBlock` (`SkeletalMeshComponent.GetAnimInstance` (`self.Mesh`)) (`self.IsBlocking`)))

(fn `UserConstructionScript`)