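; Base player Blueprint that turns attack, ability and block input into server calls and exposes stats and death state.
; Attack and ability inputs are gated on not being dead or mid-attack, with empty server events as override hooks.
; Server-side blocking applies the same gate, then messages the controller to disable movement while blocking.
; Respawning is delegated to the controller, passing the current location and player class.
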(event `Server_PrimaryAttack`
  ;[1 1 1] overrides
)

(event `Server_Ability2`
  ;[1 1 1] overrides
)

(event `Server_Ability1`
  ;[1 1 1] overrides
)

(event `InputAction|PrimaryAttack`
  (params (Key :type "Key Structure"))
  (:`Pressed`
    (if (and (not (`self.isDead`)) (not (`self.CurrentlyAttacking`)))
      (`self.Server_PrimaryAttack`))))

(event `/Game/_Main/Interfaces/INT_PlayerCharacter.RespawnCharacter`
  (message `/Game/_Main/Interfaces/INT_PlayerController.RespawnPlayer` (`self.GetController`) (`self.K2_GetActorLocation`) (`self.PlayerClass`)))

(event `InputAction|Ability1`
  (params (Key :type "Key Structure"))
  (:`Pressed`
    (if (and (not (`self.isDead`)) (not (`self.CurrentlyAttacking`)))
      (`self.Server_Ability1`))))

(event `InputAction|Block`
  (params (Key :type "Key Structure"))
  ;[1 1 1] Block
  (:`Pressed`
    (`self.Server_Blocking` true))
  (:`Released`
    (`self.Server_Blocking` false)))

(event `Server_Blocking`
  (params (Blocking :type Boolean))
  ;[1 1 1] Block
  (if (and (not (`self.isDead`)) (not (`self.CurrentlyAttacking`)))
    (set `self.IsBlocking` Blocking)
    (message `/Game/_Main/Interfaces/INT_PlayerController.SetMovementEnabled` (`self.GetController`) (not (`self.IsBlocking`)))))

(event `InputAction|Ability2`
  (params (Key :type "Key Structure"))
  (:`Pressed`
    (if (and (not (`self.isDead`)) (not (`self.CurrentlyAttacking`)))
      (`self.Server_Ability2`))))

(fn `GetPlayerStats`
  (returns (Stats :type "/Game/_Main/S_Stats Structure"))
  (return (`self.Stats`)))

(fn `PlayerDeathState`
  (returns (State :type Boolean))
  (return (`self.isDead`)))

(fn `UserConstructionScript`)